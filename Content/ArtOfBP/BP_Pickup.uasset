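; BP_Pickup is a collectible actor that comes in two variants, a tin and a button, selected by PickupType.
; The construction script sets PickUpMesh to the static mesh matching the type.
; When the first player character overlaps the Box, it calls PickedUpTin or PickedUpButton on ThirdPersonCharacter, then destroys itself.
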(event OnComponentBeginOverlap(Box)
  (params (OverlappedComponent :type Primitive%20Component%20Object%20Reference) (OtherActor :type Actor%20Object%20Reference) (OtherComp :type Primitive%20Component%20Object%20Reference) (OtherBodyIndex :type Integer) (bFromSweep :type Boolean) (SweepResult :type Hit%20Result%20Structure%20%28by%20ref%29))
  (bind _returnvalue (Game|GetPlayerCharacter 0))
  (if (== OtherActor (Game|GetPlayerCharacter 0))
    (switch int (Variables|Default|GetPickupType)
      (:0
        (bind _asthird_person_character (Utilities|Casting|CastToThirdPersonCharacter _returnvalue))
        (Default|PickedUpTin _asthird_person_character))
      (:1
        (bind _asthird_person_character_2 (Utilities|Casting|CastToThirdPersonCharacter _returnvalue))
        (Default|PickedUpButton _asthird_person_character_2)))
    (Actor|DestroyActor)))

(fn ConstructionScript
  (bind _pickupmesh (Variables|Default|GetPickUpMesh))
  (switch int (Variables|Default|GetPickupType)
    (:0
      (Components|StaticMesh|SetStaticMesh _pickupmesh "/Game/ArtOfBP/SM_Guantou.SM_Guantou"))
    (:1
      (Components|StaticMesh|SetStaticMesh _pickupmesh "/Game/ArtOfBP/SM_Button.SM_Button"))))