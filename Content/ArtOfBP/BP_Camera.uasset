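; BP_Camera is a camera actor that turns to follow the first player character, likely as a surveillance-style tracker.
; Each Tick interpolates the camera's forward vector toward the unnormalized offset to the player at a very low speed.
; The result becomes a world rotation with zero roll.
; Pitch and yaw pass through ClampAngle, but the bounds center on the new angles themselves, so the clamp never limits rotation.
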(event EventBeginPlay)

(event Collision|EventActorBeginOverlap
  (params (OtherActor :type Actor%20Object%20Reference)))

(event EventTick
  (params (DeltaSeconds :type Float%20%28single-precision%29))
  (bind _camera (Variables|Default|GetCamera))
  (Variables|Default|SetDT_DeltaTime DeltaSeconds)
  (Transformation|SetWorldRotation (Variables|Default|GetCamera) (Math|Rotator|MakeRotator 0.0 (Math|Float|ClampAngle (.Pitch (Math|Rotator|BreakRotator (Math|Rotator|MakeRotfromX (Math|Interpolation|VInterpTo (Math|Rotator|GetRotationXVector (Transformation|GetWorldRotation _camera)) (- (Transformation|GetActorLocation (Game|GetPlayerCharacter 0)) (Transformation|GetWorldLocation _camera)) (Variables|Default|GetDT_DeltaTime) 0.01)))) (- (.Pitch (Math|Rotator|BreakRotator (Math|Rotator|MakeRotfromX (Math|Interpolation|VInterpTo (Math|Rotator|GetRotationXVector (Transformation|GetWorldRotation _camera)) (- (Transformation|GetActorLocation (Game|GetPlayerCharacter 0)) (Transformation|GetWorldLocation _camera)) (Variables|Default|GetDT_DeltaTime) 0.01)))) (Math|Float|MakeLiteralFloat 8e+01)) (+ (.Pitch (Math|Rotator|BreakRotator (Math|Rotator|MakeRotfromX (Math|Interpolation|VInterpTo (Math|Rotator|GetRotationXVector (Transformation|GetWorldRotation _camera)) (- (Transformation|GetActorLocation (Game|GetPlayerCharacter 0)) (Transformation|GetWorldLocation _camera)) (Variables|Default|GetDT_DeltaTime) 0.01)))) (Math|Float|MakeLiteralFloat 8e+01))) (Math|Float|ClampAngle (.Yaw (Math|Rotator|BreakRotator (Math|Rotator|MakeRotfromX (Math|Interpolation|VInterpTo (Math|Rotator|GetRotationXVector (Transformation|GetWorldRotation _camera)) (- (Transformation|GetActorLocation (Game|GetPlayerCharacter 0)) (Transformation|GetWorldLocation _camera)) (Variables|Default|GetDT_DeltaTime) 0.01)))) (- (.Yaw (Math|Rotator|BreakRotator (Math|Rotator|MakeRotfromX (Math|Interpolation|VInterpTo (Math|Rotator|GetRotationXVector (Transformation|GetWorldRotation _camera)) (- (Transformation|GetActorLocation (Game|GetPlayerCharacter 0)) (Transformation|GetWorldLocation _camera)) (Variables|Default|GetDT_DeltaTime) 0.01)))) (Math|Float|MakeLiteralFloat 8e+01)) (+ (.Yaw (Math|Rotator|BreakRotator (Math|Rotator|MakeRotfromX (Math|Interpolation|VInterpTo (Math|Rotator|GetRotationXVector (Transformation|GetWorldRotation _camera)) (- (Transformation|GetActorLocation (Game|GetPlayerCharacter 0)) (Transformation|GetWorldLocation _camera)) (Variables|Default|GetDT_DeltaTime) 0.01)))) (Math|Float|MakeLiteralFloat 8e+01)))) false false))

(fn ConstructionScript)